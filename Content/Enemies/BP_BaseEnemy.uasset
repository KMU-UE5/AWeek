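; BP_BaseEnemy is the base enemy character, with health, melee attacks, scream, hit reactions and ragdoll death.
; A DamageSystem component handles health and raises death and damage-response events, which switch AIC_BaseEnemy between frozen, combat and dead states.
; Attacks reserve tokens from the target, tracked per target and returned when the montage ends or the enemy dies.
; Montage notifies trigger a forward sphere trace that deals damage.
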(event Custom|Initialize
  ;[0.15 0.15 0.15 0.5] Initialize
  (bind _asaic_base_enemy (Utilities|Casting|CastToAIC_BaseEnemy (AI|GetAIController self))
    (:then
      (Variables|BaseEnemy|SetAIController _asaic_base_enemy)
      (Variables|BaseEnemy|SetOriginLocation (Transformation|GetActorLocation))
      (bind _returnvalue (UserInterface|CreateWidget "/Game/Enemies/WIdget/W_HealthBar.W_HealthBar_C" 0 self))
      (UserInterface|SetWidget (Variables|Default|Getw_healthBar) _returnvalue))
    (:CastFailed
      (Development|PrintString "There is no AIC_BaseEnemy"))))

(event Custom|Death
  ;[0.15 0.15 0.15 0.5] Death
  (AI|Logic|StopLogic (Variables|/Script/AIModule.AIController|GetBrainComponent (Variables|Default|Getm_AIController)) "")
  (Components|Activation|SetActive (Variables|Default|GetCapsuleComponent) false false)
  (BaseEnemy|SetCollidertoRagdoll)
  (Default|SetStateasDead (Variables|BaseEnemy|GetAIController))
  (Rendering|SetVisibility (Variables|Default|Getw_healthBar) false true)
  (Utilities|FlowControl|Sequence
    (:then_0
      (bind _keys (Utilities|Map|Keys (Variables|BaseEnemy|GetReservedAttackTokens)))
      (for _array_element _keys
        (Class|DamageAble|ReturnAttackToken(Message) _array_element (.Value (Utilities|Map|Find (Variables|BaseEnemy|GetReservedAttackTokens) _array_element)))))
    (:then_1
      (Utilities|Time|SetTimerbyFunctionName 0 "TryCleanUp" 5.0))))

(event Custom|InitValues
  (bind _charactermovement (Variables|Character|GetCharacterMovement))
  (bind _capsulecomponent (Variables|Default|GetCapsuleComponent))
  ;[0.15 0.15 0.15 0.5] Initialize Values
  (BaseEnemy|SetMoveSpeedValue "NewEnumerator2" (Math|Random|RandomFloatinRange 4e+02 6e+02))
  (Variables|Default|SetAIControllerClass "/Game/Enemies/AIC_BaseEnemy.AIC_BaseEnemy_C")
  (Variables|/Script/Engine.NavMovementComponent|SetNavAgentProps _charactermovement (Utilities|Struct|MakeNavAgentProperties (* (Variables|/Script/Engine.CapsuleComponent|GetCapsuleRadius _capsulecomponent) 2.0) (* (Variables|/Script/Engine.CapsuleComponent|GetCapsuleHalfHeight _capsulecomponent) 2.0) -1.0 0.5 "None" false true true false false))
  (Variables|/Script/Engine.CharacterMovementComponent|SetMaxAcceleration _charactermovement 1024.0))

(event Custom|DamageResponse
  (params (DamageResponse :type EDamageResponse%20Enum :default "None"))
  ;[0.15 0.15 0.15 0.5] DamageResponse
  (Components|Movement|StopMovementImmediately (Variables|Character|GetCharacterMovement))
  (Default|SetStateasFrozen (Variables|BaseEnemy|GetAIController))
  (bind _returnvalue (Class|AWeekCharacterAnimInstance|FindRandominMontageArray (Variables|Default|Getm_AnimInstance) (Variables|Animations|GetHitReactionArrayKeyName)))
  (Variables|/Script/AWeek.DamageSystemComponent|SetIsInterruptable (Variables|Default|GetDamageSystem) false)
  (Animation|Montage|PlayMontage (Variables|Character|GetMesh) _returnvalue
    (:OnCompleted
      _)
    (:OnInterrupted
      _))
  (Variables|/Script/AWeek.DamageSystemComponent|SetIsInterruptable (Variables|Default|GetDamageSystem) true)
  (Default|SetStateasinCombat (Variables|BaseEnemy|GetAIController) (Variables|BaseEnemy|GetLastDamageSource) true))

(event EventBeginPlay
  (CallFunction|InitValues)
  (CallFunction|Initialize))

(event EventScream
  ;[0.15 0.15 0.15 0.5] Scream
  (bind _returnvalue (Class|AWeekCharacterAnimInstance|FindAnimMontage (Variables|Default|Getm_AnimInstance) (Variables|Animations|GetScreamMontageKeyName)))
  (Animation|Montage|PlayMontage (Variables|Character|GetMesh) _returnvalue
    (:OnCompleted
      _)
    (:OnInterrupted
      _))
  (Default|CallOnScreamEnd)
  (Variables|BaseEnemy|SetHasToScream false))

(event EventReturnAttackToken
  (params (Amount :type Integer))
  ;[0.15 0.15 0.15 0.5] Return Attack Token : using DamageSystem Return Attack Token
  (Class|DamageAble|ReturnAttackToken (Variables|Default|GetDamageSystem) Amount))

(event EventAttackEnd
  (params (AttackTarget :type Actor%20Object%20Reference))
  (bind _tokenusedincurrentattack (Variables|BaseEnemy|GetTokenUsedInCurrentAttack))
  ;[0.15 0.15 0.15 0.5] AttackEnd : Return the Token and Subtract the amount of token in "ReservedAttackToken"
  (Class|DamageAble|ReturnAttackToken(Message) AttackTarget _tokenusedincurrentattack)
  (CallFunction|StoreAttackTokens AttackTarget (* _tokenusedincurrentattack -1))
  (Default|CallOnAttackEnd)
  (Variables|BaseEnemy|Setis%20Attacking false))

(event EventStoreAttackTokens
  (params (AttackTarget :type Actor%20Object%20Reference) (Amount :type Integer))
  (bind _reservedattacktokens (Variables|BaseEnemy|GetReservedAttackTokens))
  (bind (_value _returnvalue) (Utilities|Map|Find _reservedattacktokens AttackTarget))
  ;[0.15 0.15 0.15 0.5] StoreAttackTokens : Store the Token in the "ReservedAttackToken" TMap<TObjectPtr<AActor>, int>
  (Utilities|Map|Add (Variables|BaseEnemy|GetReservedAttackTokens) AttackTarget (Math|Integer|SelectInt (+ _value Amount) Amount _returnvalue)))

(event EventDefaultAttack
  (params (AttackTarget :type Actor%20Object%20Reference))
  ;[0.15 0.15 0.15 0.5] Default Attack
  (if (not (Variables|/Script/AWeek.DamageSystemComponent|GetIsDead (Variables|Default|GetDamageSystem)))
    (Variables|BaseEnemy|Setis%20Attacking true)
    (bind _returnvalue (Class|AWeekCharacterAnimInstance|FindRandominMontageArray (Variables|Default|Getm_AnimInstance) (Variables|Animations|GetAttackArrayKeyName)))
    (Variables|/Script/AWeek.DamageSystemComponent|SetIsInterruptable (Variables|Default|GetDamageSystem) false)
    (bind _notifyname (Animation|Montage|PlayMontage (Variables|Character|GetMesh) _returnvalue)
      (:OnCompleted
        (CallFunction|AttackEnd AttackTarget :!label _label)
        (Variables|/Script/AWeek.DamageSystemComponent|SetIsInterruptable (Variables|Default|GetDamageSystem) true))
      (:OnInterrupted
        (goto _label))
      (:OnNotifyBegin
        (switch name _notifyname
          (:Smash
            (bind _hitactor (BaseEnemy|ForwardAttackCollision false))
            (Utilities|IsValid _hitactor
              (:Is%20Valid
                (Class|DamageAble|TakeDamage(Message) _hitactor (Utilities|Struct|MakeDamageInfo 1e+01 "Default"))))))))))

(fn ConstructionScript
  (bind _damagesystem (Variables|Default|GetDamageSystem))
  (EventDispatchers|BindEventtoOnDeath _damagesystem (EventDispatchers|CreateEvent :!event Custom|Death))
  (EventDispatchers|BindEventtoOnDamageResponse _damagesystem (EventDispatchers|CreateEvent :!event Custom|DamageResponse)))

(fn TakeDamage
  (params (DamageInfo :type Damage%20Info%20Structure))
  (Variables|BaseEnemy|SetLastDamageSource (.DamageSource (Utilities|Struct|BreakDamageInfo DamageInfo)))
  (Class|DamageAble|TakeDamage (Variables|Default|GetDamageSystem) DamageInfo)
  (return false))

(fn Heal
  (params (amount :type Float%20%28single-precision%29))
  (bind _returnvalue (Class|DamageAble|Heal (Variables|Default|GetDamageSystem) amount))
  (return _returnvalue))

(fn GetMaxHealth
  (return (Class|DamageAble|GetMaxHealth (Variables|Default|GetDamageSystem))))

(fn GetCurrentHealth
  (return (Class|DamageAble|GetCurrentHealth (Variables|Default|GetDamageSystem))))

(fn ForwardAttackCollision
  (params (IgnoreSelfType :type Boolean))
  (bind _returnvalue (Transformation|GetActorLocation))
  (LocalVariables|SetSelfTypeIgnore IgnoreSelfType)
  (bind (_outhit _returnvalue_2) (Collision|SphereTraceForObjects _returnvalue (+ _returnvalue (* (Transformation|GetActorForwardVector) 2e+02)) 2e+01 (Utilities|Array|MakeArray "ObjectTypeQuery3") false 0 "ForDuration"))
  (if _returnvalue_2
    (if (LocalVariables|GetSelfTypeIgnore)
      (Utilities|Casting|CastToBP_BaseEnemy (.HitActor (Collision|BreakHitResult _outhit))
        (:CastFailed
          (return (.HitActor (Collision|BreakHitResult _outhit)))))
      (else
        (return (.HitActor (Collision|BreakHitResult _outhit)))))))

(fn SetCollidertoRagdoll
  (bind _mesh (Variables|Character|GetMesh))
  (Collision|SetCollisionProfileName _mesh "Ragdoll" true :!class /Script/Engine.PrimitiveComponent)
  (Physics|SetSimulatePhysics _mesh true)
  (Collision|SetCollisionEnabled _mesh "QueryAndPhysics")
  (Collision|SetCollisionResponsetoChannel _mesh "ECC_Pawn" "ECR_Ignore")
  (Collision|SetCollisionResponsetoChannel _mesh "ECC_Camera" "ECR_Ignore"))

(fn GetIsDead
  (bind _returnvalue (Class|DamageAble|GetIsDead (Variables|Default|GetDamageSystem)))
  (return _returnvalue))

(fn ReserveAttackToken
  (params (Amount :type Integer))
  (bind _returnvalue (Class|DamageAble|ReserveAttackToken (Variables|Default|GetDamageSystem) Amount))
  (return _returnvalue))

(fn SetMoveSpeedValue
  (params (EMoveType :type E_MovementType%20Enum :default "NewEnumerator0") (Speed :type Float%20%28double-precision%29))
  (Utilities|Map|Add (Variables|BaseEnemy|GetMovementSpeeds) EMoveType Speed))

(fn TryCleanUp
  (Rendering|SetActorHiddenInGame true)
  (Physics|SetSimulatePhysics (Variables|Character|GetMesh) false)
  (Collision|SetCollisionEnabled (Variables|Character|GetMesh) "NoCollision")
  (Actor|DestroyActor))

(fn AttackStart
  (params (AttackTarget :type Actor%20Object%20Reference) (TokenNeeded :type Integer))
  (bind _returnvalue (Class|DamageAble|ReserveAttackToken(Message) AttackTarget TokenNeeded))
  (if _returnvalue
    (CallFunction|StoreAttackTokens AttackTarget TokenNeeded)
    (Variables|BaseEnemy|SetTokenUsedInCurrentAttack TokenNeeded)
    (return true)
    (else
      (return false))))

(fn GetIdealRange
  (return (Variables|BaseEnemy|GetAttack%20Radius) (Variables|BaseEnemy|GetDefend%20Radius)))

(fn GetMovementSpeed
  (params (MovmentType :type E_MovementType%20Enum :default "NewEnumerator0"))
  (return (.Value (Utilities|Map|Find (Variables|BaseEnemy|GetMovementSpeeds) MovmentType))))

(fn GetPatrolRoute
  (return (Variables|BaseEnemy|GetPatrolRoute)))

(fn SetMovementSpeed
  (params (MovementType :type E_MovementType%20Enum :default "NewEnumerator0"))
  (bind _output_get (Variables|/Script/Engine.CharacterMovementComponent|SetMaxWalkSpeed (Variables|Character|GetCharacterMovement) (.Value (Utilities|Map|Find (Variables|BaseEnemy|GetMovementSpeeds) MovementType))))
  (return _output_get))