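; Test player character for exercising enemy AI, with a damageable interface, a health bar and a debug attack.
; Health, death, damage and attack-token calls forward to DamageSystem1, while Heal is a stub returning zero.
; T runs a short forward sphere trace that damages the hit actor and reports a damage event to AI perception.
; Zoom input drives a timeline that blends the camera boom into an over-the-shoulder offset.
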(event Input|EnhancedActionEvents|EnhancedInputActionIA_Zoom
  (params (ActionValue :type Boolean) (ElapsedSeconds :type Float%20%28double-precision%29) (TriggeredSeconds :type Float%20%28double-precision%29) (InputAction :type Input%20Action%20Object%20Reference :default "/Game/Player/Input/Actions/IA_Zoom.IA_Zoom"))
  (:Started
    (bind _maintrack (Timeline|ZoomTimline Play)
      (:Update
        (Variables|/Script/Engine.SpringArmComponent|SetTargetArmLength (Variables|Default|GetCameraBoom) (Math|Float|Lerp 4e+02 2.5e+02 _maintrack))
        (Variables|/Script/Engine.SpringArmComponent|SetSocketOffset (Variables|Default|GetCameraBoom) (Math|Vector|MakeVector 0.0 (Math|Float|Lerp 0.0 1e+02 _maintrack) (Math|Float|Lerp 0.0 3e+01 _maintrack))))))
  (:Completed
    (Timeline|ZoomTimline Reverse)))

(event EventReturnAttackToken
  (params (Amount :type Integer))
  (Class|DamageAble|ReturnAttackToken (Variables|Default|GetDamageSystem1) Amount))

(event EventBeginPlay
  (Utilities|FlowControl|Delay 0.5)
  (bind _returnvalue (UserInterface|CreateWidget "/Game/Enemies/WIdget/W_HealthBar.W_HealthBar_C" 0 self))
  (UserInterface|SetWidget (Variables|Default|Getw_healthbar) _returnvalue))

(event Input|KeyboardEvents|T
  (params (Key :type Key%20Structure :default "None"))
  (bind _returnvalue (Transformation|GetActorLocation))
  (:Pressed
    (bind (_outhit _returnvalue_2) (Collision|SphereTraceForObjects _returnvalue (+ _returnvalue (* (Transformation|GetActorForwardVector) 1e+02)) 2e+01 (Utilities|Array|MakeArray "ObjectTypeQuery9") false 0 "ForDuration" true "(R=1.000000,G=0.000000,B=0.000000,A=1.000000)" "(R=0.000000,G=1.000000,B=0.000000,A=1.000000)" 0.5))
    (if _returnvalue_2
      (Class|DamageAble|TakeDamage(Message) (.HitActor (Collision|BreakHitResult _outhit)) (Utilities|Struct|MakeDamageInfo 1e+01 "Default" "None" false false false false self (Utilities|Struct|MakeDamageHitInfo (.ImpactPoint (Collision|BreakHitResult _outhit)) (.ImpactNormal (Collision|BreakHitResult _outhit)) (.HitComponent (Collision|BreakHitResult _outhit)) (.HitBoneName (Collision|BreakHitResult _outhit)))))
      (Development|PrintString (Utilities|GetObjectName (.HitActor (Collision|BreakHitResult _outhit))))
      (Class|AISenseDamage|ReportDamageEvent (.HitActor (Collision|BreakHitResult _outhit)) self 1.0 (Transformation|GetActorLocation) "0, 0, 0" "None"))))

(fn ConstructionScript)

(fn TakeDamage
  (params (DamageInfo :type Damage%20Info%20Structure))
  (bind _returnvalue (Class|DamageAble|TakeDamage (Variables|Default|GetDamageSystem1) DamageInfo))
  (return _returnvalue))

(fn Heal
  (params (amount :type Float%20%28single-precision%29))
  (return 0.0))

(fn GetMaxHealth
  (return (Class|DamageAble|GetMaxHealth (Variables|Default|GetDamageSystem1))))

(fn GetCurrentHealth
  (return (Class|DamageAble|GetCurrentHealth (Variables|Default|GetDamageSystem1))))

(fn GetIsDead
  (return (Variables|/Script/AWeek.DamageSystemComponent|GetIsDead (Variables|Default|GetDamageSystem1))))

(fn ReserveAttackToken
  (params (Amount :type Integer))
  (bind _returnvalue (Class|DamageAble|ReserveAttackToken (Variables|Default|GetDamageSystem1) Amount))
  (return _returnvalue))