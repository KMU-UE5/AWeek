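; Player character Blueprint that handles zoom input, damage and health calls, and hit and death animations.
; IA_Zoom plays or reverses a timeline that pulls the camera boom in over the shoulder, broadcasting ZoomIn/ZoomOut gameplay messages.
; Health, damage and attack-token functions forward to MDamageSystem, though GetIsDead always returns false and ReserveAttackToken passes zero instead of its Amount.
; Die and OnHit play montages, the latter only for Hit Reaction responses.
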(event Input|EnhancedActionEvents|EnhancedInputActionIA_Zoom
  (params (ActionValue :type Boolean) (ElapsedSeconds :type Float%20%28double-precision%29) (TriggeredSeconds :type Float%20%28double-precision%29) (InputAction :type Input%20Action%20Object%20Reference :default "/Game/Player/Input/Actions/IA_Zoom.IA_Zoom"))
  (bind _returnvalue (Subsystems|GetGameEventMessageSubsystem))
  (bind _rigvmfunction_mathintmake (Utilities|Struct|MakeRigVMFunction_MathIntMake))
  (:Started
    (Class|GameEventMessageSubsystem|BroadcastMessage _returnvalue "(TagName=\"Event.Weapon.ZoomIn\")" _rigvmfunction_mathintmake)
    (bind _maintrack (Timeline|ZoomTimline Play)
      (:Update
        (Variables|/Script/Engine.SpringArmComponent|SetTargetArmLength (Variables|Default|GetCameraBoom) (Math|Float|Lerp 4e+02 2.5e+02 _maintrack))
        (Variables|/Script/Engine.SpringArmComponent|SetSocketOffset (Variables|Default|GetCameraBoom) (Math|Vector|MakeVector 0.0 (Math|Float|Lerp 0.0 1e+02 _maintrack) (Math|Float|Lerp 0.0 3e+01 _maintrack))))))
  (:Completed
    (Class|GameEventMessageSubsystem|BroadcastMessage _returnvalue "(TagName=\"Event.Weapon.ZoomOut\")" _rigvmfunction_mathintmake)
    (Timeline|ZoomTimline Reverse)))

(event EventReturnAttackToken
  (params (Amount :type Integer))
  (Class|DamageAble|ReturnAttackToken (Variables|Default|GetmDamageSystem) Amount))

(event EventDie
  (Animation|Montage|PlayMontage (Variables|Character|GetMesh) "/Game/Player/Animation/Montages/AM_Die.AM_Die"))

(event EventOnHit
  (params (Response :type EDamageResponse%20Enum :default "None"))
  (switch Utilities|FlowControl|Switch|SwitchonEDamageResponse Response
    (:HitReaction
      (Animation|Montage|PlayMontage (Variables|Character|GetMesh) "/Game/Player/Animation/AM_Hit.AM_Hit"))))

(fn ConstructionScript)

(fn ReserveAttackToken
  (params (Amount :type Integer))
  (bind _returnvalue (Class|DamageAble|ReserveAttackToken (Variables|Default|GetmDamageSystem)))
  (return _returnvalue))

(fn TakeDamage
  (params (DamageInfo :type Damage%20Info%20Structure))
  (bind _returnvalue (Class|DamageAble|TakeDamage (Variables|Default|GetmDamageSystem) DamageInfo))
  (return _returnvalue))

(fn Heal
  (params (amount :type Float%20%28single-precision%29))
  (bind _returnvalue (Class|DamageAble|Heal (Variables|Default|GetmDamageSystem) amount))
  (return _returnvalue))

(fn GetMaxHealth
  (return (Class|DamageAble|GetMaxHealth (Variables|Default|GetmDamageSystem))))

(fn GetIsDead
  (return false))

(fn GetCurrentHealth
  (return (Class|DamageAble|GetCurrentHealth (Variables|Default|GetmDamageSystem))))